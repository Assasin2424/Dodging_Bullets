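; Turret actor that tracks the player and fires hitscan shots until killed.
; Once PlayerM_CH enters the Cone, a Delay loop turns the head smoothly toward them and calls Shoot, continuing until death with no end-overlap check.
; Shoot line-traces forward from Scene and damages the hit actor, rate-limited by WeaponReady.
; AnyDamage drains Health; at zero the meshes simulate physics, a particle effect spawns, and the actor is destroyed shortly after.
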(event OnComponentBeginOverlap(Cone)
  (params (OverlappedComponent :type Primitive%20Component%20Object%20Reference) (OtherActor :type Actor%20Object%20Reference) (OtherComp :type Primitive%20Component%20Object%20Reference) (OtherBodyIndex :type Integer) (bFromSweep :type Boolean) (SweepResult :type Hit%20Result%20Structure%20%28by%20ref%29))
  ;[1 1 1] Look At
  (bind _asplayer_m_ch (Utilities|Casting|CastToPlayerM_CH OtherActor))
  (if (Variables|Default|GetAlive?)
    (CallFunction|UpdateTurretHeadRotation _asplayer_m_ch :!label _label)
    (Utilities|FlowControl|Sequence
      (:then_0
        (CallFunction|Shoot))
      (:then_1
        (Utilities|FlowControl|Delay 0.001)
        (if (Variables|Default|GetAlive?)
          (goto _label))))))

(event Custom|Shoot
  (bind _scene (Variables|Default|GetScene))
  (bind _returnvalue (Transformation|GetWorldLocation _scene))
  ;[1 1 1] Shooting
  (if (and (Variables|Default|GetWeapon%20Ready) (Variables|Default|GetAlive?))
    (bind _outhit (Collision|LineTraceByChannel _returnvalue (+ _returnvalue (* (Math|Vector|GetForwardVector _scene) 3e+03)) "TraceTypeQuery1" false 0 "ForDuration" true "(R=1.000000,G=0.000000,B=0.000000,A=1.000000)" "(R=0.000000,G=1.000000,B=0.000000,A=1.000000)" 4.5))
    (Utilities|FlowControl|Sequence
      (:then_0
        (Variables|Default|SetWeapon%20Ready false)
        (Utilities|FlowControl|Delay 0.2)
        (Variables|Default|SetWeapon%20Ready true))
      (:then_1
        (Game|Damage|ApplyDamage (.HitActor (Collision|BreakHitResult _outhit)) 15.0 (Game|GetPlayerController 0) self)))))

(event Game|Damage|EventAnyDamage
  (params (Damage :type Float%20%28single-precision%29) (DamageType :type Damage%20Type%20Object%20Reference) (InstigatedBy :type Controller%20Object%20Reference) (DamageCauser :type Actor%20Object%20Reference))
  ;[1 1 1] Health System
  (if (and (<= (Variables|Default|GetHealth) 0.0) (Variables|Default|GetAlive?))
    (Physics|SetSimulatePhysics (Variables|Default|GetCube) true :!label _label)
    (Variables|Default|SetAlive? false)
    (AddComponent|AddParticleSystemComponent false)
    (Utilities|FlowControl|Delay 3.0)
    (Actor|DestroyActor)
    (else
      (Variables|Default|SetHealth (- (Variables|Default|GetHealth) Damage))
      (if (and (<= (Variables|Default|GetHealth) 0.0) (Variables|Default|GetAlive?))
        (goto _label)))))

(fn ConstructionScript)

(fn UpdateTurretHeadRotation
  (params (Target :type Actor%20Object%20Reference))
  (Transformation|SetWorldRotation (Variables|Default|GetCube) (Math|Interpolation|RInterpTo (Transformation|GetWorldRotation (Variables|Default|GetCube)) (Math|Rotator|FindRelativeLookatRotation (Transformation|GetActorTransform) (Transformation|GetActorLocation Target)) (Utilities|Time|GetWorldDeltaSeconds) 1e+01) false false))