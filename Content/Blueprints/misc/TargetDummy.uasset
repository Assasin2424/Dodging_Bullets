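; TargetDummy is a damageable dummy that ragdolls when killed and then removes itself.
; AnyDamage subtracts incoming damage from Health, and when none remains it disables capsule collision and enables physics simulation on the mesh.
; After a brief delay the mesh collision becomes physics-only, and a longer delay precedes destroying the actor.
; Damage received at zero or lower Health also enters this death sequence.
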(event Game|Damage|EventAnyDamage
  (params (Damage :type Float%20%28single-precision%29) (DamageType :type Damage%20Type%20Object%20Reference) (InstigatedBy :type Controller%20Object%20Reference) (DamageCauser :type Actor%20Object%20Reference))
  (bind _mesh (Variables|Character|GetMesh))
  ;[1 1 1] Health/Death System
  (if (> (Variables|Default|GetHealth) 0.0)
    (Variables|Default|SetHealth (- (Variables|Default|GetHealth) Damage))
    (if (not (> (Variables|Default|GetHealth) 0.0))
      (Collision|SetCollisionEnabled (Variables|Collision|GetCapsuleComponent) "NoCollision" :!label _label)
      (Physics|SetSimulatePhysics _mesh true)
      (Utilities|FlowControl|Delay 0.2)
      (Collision|SetCollisionEnabled _mesh "PhysicsOnly")
      (Utilities|FlowControl|Delay 5.0)
      (Actor|DestroyActor))
    (else
      (goto _label))))

(fn ConstructionScript)