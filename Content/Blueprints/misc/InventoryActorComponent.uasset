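; InventoryActorComponent is an inventory component that stores and equips weapons for a character.
; InitalizeInventory caches the owning character, which EquipWeapon passes to the weapon through InitalizeWeaponMessage before attaching it to the GripPoint socket on the PlayerM_CH arms.
; StoreWeapon clears the inventory before adding, so it holds only one weapon at a time.
; HideWeapon is an empty stub, and the weapon index inputs are unused.
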(fn EquipWeapon
  (params (Weapon :type Actor%20Object%20Reference) (Weapon%20Int%200 :type Integer))
  (bind _character (Variables|Default|GetCharacter))
  (Class|WeaponInterface|InitalizeWeapon(Message) Weapon _character)
  (bind _asplayer_m_ch (Utilities|Casting|CastToPlayerM_CH _character))
  (Transformation|AttachComponentToComponent Weapon (Variables|/Game/Blueprints/Player/Main/PlayerM_CH.PlayerM_CH_C|GetArms _asplayer_m_ch) "GripPoint" "KeepRelative" "KeepRelative" "KeepRelative" true)
  (return false))

(fn HideWeapon
  (params (Weapon :type Actor%20Object%20Reference) (Weapon%20Int%200 :type Integer))
  (return false))

(fn InitalizeInventory
  (params (Character :type Character%20Object%20Reference))
  (Variables|Default|SetCharacter Character)
  (return false))

(fn StoreWeapon
  (params (Weapon :type Actor%20Object%20Reference) (Weapon%20Int%200 :type Integer))
  (bind _inventory (Variables|Default|GetInventory))
  (Utilities|Array|Clear _inventory)
  (Utilities|Array|AddUnique _inventory Weapon)
  (return false))